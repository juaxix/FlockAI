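; Flocking agent Blueprint that holds boids-style steering logic, currently disconnected: CalculateNewMoveVector is empty and the computation never runs.
; The unwired graph derives alignment, cohesion and separation from agents overlapping VisionSphere.
; It sums repulsion from negative Stimulus actors, rescaled to the strongest, and picks the positive one with the best value-to-distance ratio.
; Weighted flocking terms plus both stimulus vectors form NewMoveVector; debug printing is also unwired.
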(event EventCalculateNewMoveVector)

(fn ConstructionScript)

(fn ResetComponents
  (Variables|AI|SetAlignmentComponent "0, 0, 0")
  (Variables|AI|SetCohesionComponent "0, 0, 0")
  (Variables|AI|SetSeparationComponent "0, 0, 0")
  (Variables|AI|SetNegativeStimuliComponent "0, 0, 0")
  (Variables|AI|SetNegativeStimuliMaxFactor 0.0)
  (Variables|AI|SetPositiveStimuliComponent "0, 0, 0")
  (Variables|AI|SetPositiveStimuliMaxFactor 0.0))

(fn DebugComponents)